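; BP_TerrainGen is a world-generation actor that lays out a flat, square grid of ground mesh instances centered on the world origin.
; PopulateGrid fills GridArray with positions from GridSize and WorldGridSize, offset to center the grid.
; HismPop rebuilds the GroundMeshes instances from that array in world space at a fixed scale, while ClearHism removes them and Debug draws spheres at each point.
; The event graph and construction script are empty, so nothing here calls these functions.
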(fn `ClearHism`
  (`InstancedStaticMeshComponent.ClearInstances` (`self.GroundMeshes`)))

(fn `Debug`
  (for _array_element (`self.GridArray`)
    (`KismetSystemLibrary.DrawDebugSphere` _array_element 100.0 12 (struct :`R` 1.0 :`G` 1.0 :`B` 1.0 :`A` 1.0) 1.0 10.0)))

(fn `HismPop`
  (`InstancedStaticMeshComponent.ClearInstances` (`self.GroundMeshes`))
  (for _array_element (`self.GridArray`)
    (`InstancedStaticMeshComponent.AddInstance` (`self.GroundMeshes`) (`KismetMathLibrary.MakeTransform` _array_element (struct) (2.0 2.0 2.0)) true)))

(fn `PopulateGrid`
  (bind _worldgridsize (`self.WorldGridSize`))
  (bind _worldgridsize_2 (`self.WorldGridSize`))
  (bind _returnvalue (`KismetMathLibrary.FTrunc` (`self.WorldOffset`)))
  (`KismetArrayLibrary.Array_Clear` (`self.GridArray`))
  (set `self.WorldOffset` (- (* (* (`self.GridSize`) _worldgridsize) 0.5) (* _worldgridsize 0.5)))
  ;[1 1 1] Y loop
  (for _index (range (`self.GridSize`))
    ;[1 1 1] X loop
    (for _index_2 (range (`self.GridSize`))
      (`KismetArrayLibrary.Array_Add` (`self.GridArray`) (`KismetMathLibrary.MakeVector` (`KismetMathLibrary.Conv_IntToDouble` (- (* _index_2 _worldgridsize_2) _returnvalue)) (`KismetMathLibrary.Conv_IntToDouble` (- (* _worldgridsize_2 _index) _returnvalue)))))))

(fn `UserConstructionScript`)