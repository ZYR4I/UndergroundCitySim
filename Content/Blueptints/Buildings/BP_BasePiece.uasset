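; Base building piece that snaps itself to the nearest point of a referenced grid and clears the wall tiles it overlaps.
; On BeginPlay it spawns a BP_AiHandler at Box1 and starts a short looping timer.
; Each tick of the timer moves the piece to the closest grid point and destroys overlapping BP_EnhancedWallCollision tiles, stopping once none overlap.
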(event `self.ReceiveBeginPlay`
  (bind _returnvalue (`KismetSystemLibrary.K2_SetTimerDelegate` (delegate `AllignToGrid`) 0.1 true))
  (set `self.SpawnTimerHandle` _returnvalue)
  (`|SpawnActorFromClass` "/Game/Blueptints/Ai/BP_AiHandler.BP_AiHandler_C" (`KismetMathLibrary.MakeTransform` (`SceneComponent.K2_GetComponentLocation` (`self.Box1`))) "Undefined" "MultiplyWithRoot" null null))

(event `AllignToGrid`
  (bind _closestpoint1 (`self.Get Closest Grid Point`))
  (`self.K2_SetActorLocation` (`|GetArrayItem` (`MyTerrainGen.gridPoints` (`self.GridRef`)) _closestpoint1))
  (`self.DestroyWallTiles`))

(event `DestroyWallTiles`
  (`self.DestroyWalls`))

(fn `DestroyWalls`
  (bind _overlappingactors (`self.GetOverlappingActors` "/Game/Blueptints/WorldGen/BP_EnhancedWallCollision.BP_EnhancedWallCollision_C"))
  (if (!= (`KismetArrayLibrary.Array_Length` _overlappingactors) 0)
    (for _array_element _overlappingactors
      (bind _asbp_enhanced_wall_collision (cast `/Game/Blueptints/WorldGen/BP_EnhancedWallCollision` _array_element))
      (`/Game/Blueptints/WorldGen/BP_EnhancedWallCollision.DestroyWallTile` _asbp_enhanced_wall_collision))
    (else
      (`KismetSystemLibrary.K2_ClearAndInvalidateTimerHandle` (`self.SpawnTimerHandle`)))))

(fn `Get Closest Grid Point`
  (returns (ClosestPoint1 :type Integer))
  (locals (ClosestPoint :type Integer) (ClosestDistance :type "Float (double-precision)" :default 999.0))
  (for (_array_element _array_index) (`MyTerrainGen.gridPoints` (`self.GridRef`))
    (bind _returnvalue (`KismetMathLibrary.Vector_Distance` _array_element (`self.K2_GetActorLocation`)))
    (if (< _returnvalue (`local.ClosestDistance`))
      (set `local.ClosestPoint` _array_index)
      (set `local.ClosestDistance` _returnvalue)))
  (return (`local.ClosestPoint`)))

(fn `UserConstructionScript`)