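; BP_AiHandler manages a queue of walls marked for demolition and dispatches it to AI workers, spawning one BP_Worker on BeginPlay.
; Player interaction with an enhanced wall collision toggles that wall in TaskQueue, recolors it through DestructionHandler, then assigns or clears work on every worker.
; WorkerDestroyedWall dequeues a wall and has DestructionHandler destroy it.
; Debug prints show the queue length each tick and each removal result.
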(event `self.ReceiveBeginPlay`
  (bind _returnvalue (`|SpawnActorFromClass` "/Game/Blueptints/Ai/BP_Worker.BP_Worker_C" (`self.GetTransform`) "AlwaysSpawn" "MultiplyWithRoot" null self null))
  (`KismetArrayLibrary.Array_Add` (`self.WorkerRef`) _returnvalue)
  (bind _asbp_player_character (cast `/Game/Blueptints/Player/BP_PlayerCharacter` (`GameplayStatics.GetPlayerCharacter` 0)))
  (add `/Game/Blueptints/Player/BP_PlayerCharacter.Interaction` _asbp_player_character (delegate `PlayerInterated`)))

(event `PlayerInterated`
  (bind _asbp_enhanced_wall_collision (cast `/Game/Blueptints/WorldGen/BP_EnhancedWallCollision` (`/Game/Blueptints/Player/BP_PlayerCharacter.TargetedActor` (stale `self.ReceiveBeginPlay` _asbp_player_character))))
  (`self.WallClicked` _asbp_enhanced_wall_collision))

(event `self.ReceiveTick`
  (params (DeltaSeconds :type "Float (single-precision)"))
  (`KismetSystemLibrary.PrintString` (`KismetStringLibrary.Conv_IntToString` (`KismetArrayLibrary.Array_Length` (`self.TaskQueue`))) true true (struct :`G` 0.66 :`B` 1.0 :`A` 1.0) DeltaSeconds))

(fn `UpdateWorker`
  (params (IsWork :type Boolean))
  (for _array_element (`self.WorkerRef`)
    (if IsWork
      (`/Game/Blueptints/Ai/BP_Worker.WorkAssigned` _array_element (`self.TaskQueue`))
      (else
        (`/Game/Blueptints/Ai/BP_Worker.NoWorkAssigned` _array_element))))
  (return))

(fn `UserConstructionScript`)

(fn `WallClicked`
  (params (WallRef :type "/Game/Blueptints/WorldGen/BP_EnhancedWallCollision Object Reference"))
  (bind _wallref (`local.WallRef`))
  (bind _wallref_2 (`local.WallRef`))
  (if (== (`KismetArrayLibrary.Array_Find` (`self.TaskQueue`) WallRef) -1)
    (`/Game/Blueptints/WorldGen/BP_DestructionHandler.SetWallColor` (`self.DestructionHandler`) _wallref true)
    (`KismetArrayLibrary.Array_AddUnique` (`self.TaskQueue`) _wallref)
    (else
      (`/Game/Blueptints/WorldGen/BP_DestructionHandler.SetWallColor` (`self.DestructionHandler`) _wallref_2 false)
      (`KismetArrayLibrary.Array_RemoveItem` (`self.TaskQueue`) _wallref_2)))
  (`self.UpdateWorker` (> (`KismetArrayLibrary.Array_Length` (`self.TaskQueue`)) 0))
  (return))

(fn `WorkerDestroyedWall`
  (params (WallRef :type "/Game/Blueptints/WorldGen/BP_EnhancedWallCollision Object Reference"))
  (returns (Removed :type Boolean))
  (bind _returnvalue (`KismetArrayLibrary.Array_RemoveItem` (`self.TaskQueue`) (`local.WallRef`)))
  (bind _returnvalue_2 (`/Game/Blueptints/WorldGen/BP_DestructionHandler.DestroyWall` (`self.DestructionHandler`) WallRef))
  (`KismetSystemLibrary.PrintString` (`KismetMathLibrary.SelectString` "Removed" "NotRemoved" (and _returnvalue_2 _returnvalue)) true true (struct :`R` 1.0 :`G` 0.028182 :`A` 1.0))
  (return _returnvalue_2))