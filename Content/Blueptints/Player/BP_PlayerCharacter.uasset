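; Player character with an orbiting, zoomable spring arm camera and mouse-driven interaction with world actors.
; Movement follows flattened camera vectors, while camera events yaw the spring arm and adjust its clamped length.
; Each tick, a line trace from the deprojected cursor stores any hit actor implementing BPI_PlayerInteraction as TargetedActor.
; Click sends that actor the InteractedMessage interface call, passing the character.
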(event `ZoomCamera`
  (params (Axis :type "Float (double-precision)"))
  (set `SpringArmComponent.TargetArmLength` (`KismetMathLibrary.FClamp` (+ (* Axis 30.0) (`SpringArmComponent.TargetArmLength` (`self.SpringArm`))) 400.0 1500.0) (`self.SpringArm`)))

(event `Move`
  (params (X :type "Float (double-precision)") (Y :type "Float (double-precision)"))
  (bind (_returnvalue _returnvalue2) (`self.F&RVector`))
  (`self.AddMovementInput` _returnvalue X)
  (`self.AddMovementInput` _returnvalue2 Y))

(event `RotateCamera`
  (params (`Delta Rotation Z (Yaw)` :type "Float (single-precision)"))
  (`SceneComponent.K2_AddWorldRotation` (`self.SpringArm`) (`KismetMathLibrary.MakeRotator` 0.0 0.0 `Delta Rotation Z (Yaw)`) false false))

(event `Click`
  (message `/Game/Blueptints/Interfaces/BPI_PlayerInteraction.Interacted` (`self.TargetedActor`) self))

(event `self.ReceiveTick`
  (params (DeltaSeconds :type "Float (single-precision)"))
  (`self.PlayerTrace` "None"))

(fn `PlayerTrace`
  (params (DrawDebugType :type "EDrawDebugTrace Enum" :default "None"))
  (bind (_worldlocation _worlddirection) (`PlayerController.DeprojectMousePositionToWorld` (`GameplayStatics.GetPlayerController` 0)))
  (bind _outhit (`KismetSystemLibrary.LineTraceSingle` :`Start` _worldlocation :`End` (+ _worldlocation (* _worlddirection 3000.0)) :`TraceChannel` "TraceTypeQuery3" :`DrawDebugType` DrawDebugType :`DrawTime` 1.0))
  (bind (_bblockinghit _binitialoverlap _time _distance _location _impactpoint _normal _impactnormal _physmat _hitactor) (`GameplayStatics.BreakHitResult` _outhit))
  (if (and _bblockinghit (`KismetSystemLibrary.DoesImplementInterface` _hitactor "/Game/Blueptints/Interfaces/BPI_PlayerInteraction.BPI_PlayerInteraction_C"))
    (set `self.TargetedActor` _hitactor)
    (else
      (set `self.TargetedActor` null))))

(fn `UserConstructionScript`)