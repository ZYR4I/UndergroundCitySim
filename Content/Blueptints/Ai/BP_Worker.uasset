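; BP_Worker is an AI worker that takes a list of wall tasks and targets the nearest one.
; Interact box-traces ahead and reports a hit on the current wall to AiHandler as destroyed, otherwise it re-picks the nearest task.
; NotValidTask steps through the task list, falling back to a no-work state on an invalid entry.
; State changes are pushed to the controller, and Tick prints debug info.
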(event `Interact`
  (bind _returnvalue (`self.K2_GetActorLocation`))
  (bind _outhit (`KismetSystemLibrary.BoxTraceSingle` :`Start` _returnvalue :`End` (+ _returnvalue (* (`self.GetActorForwardVector`) 150.0)) :`HalfSize` (20.0 20.0 50.0) :`TraceChannel` "TraceTypeQuery3" :`DrawDebugType` "ForDuration"))
  (bind (_bblockinghit _binitialoverlap _time _distance _location _impactpoint _normal _impactnormal _physmat _hitactor) (`GameplayStatics.BreakHitResult` _outhit))
  (if (== _hitactor (`self.CurrentTask`))
    (bind _asbp_enhanced_wall_collision (cast `/Game/Blueptints/WorldGen/BP_EnhancedWallCollision` _hitactor))
    (`/Game/Blueptints/Ai/BP_AiHandler.WorkerDestroyedWall` (`self.AiHandler`) _asbp_enhanced_wall_collision)
    (else
      (`self.GetNearestWall`))))

(event `NotValidTask`
  (bind _taskfinderindex (`self.TaskFinderIndex`))
  (if (> (`self.TaskFinderIndex`) (`KismetArrayLibrary.Array_Length` (`self.PotentialTasks`)))
    (set `self.TaskFinderIndex` 0)
    (else
      (`/Engine/EditorBlueprintResources/StandardMacros.IncrementInt` _taskfinderindex
        (:`  `
          _))))
  (bind _output_get (set `self.CurrentTask` (`|GetArrayItem` (`self.PotentialTasks`) _taskfinderindex)))
  (`self.SetWorking`)
  (`/Engine/EditorBlueprintResources/StandardMacros.IsValid` _output_get
    (:`Is Not Valid`
      (`self.NoWorkAssigned`))))

(event `NoWorkAssigned`
  (bind _output_get (set `self.AiState` "NewEnumerator0"))
  (`/Game/Blueptints/Ai/BP_AiController.StateUpdate` (`self.ControllerRef`) _output_get))

(event `SetWorking`
  (bind _output_get (set `self.AiState` "NewEnumerator1"))
  (`/Game/Blueptints/Ai/BP_AiController.StateUpdate` (`self.ControllerRef`) _output_get))

(event `self.ReceiveTick`
  (params (DeltaSeconds :type "Float (single-precision)"))
  (`KismetSystemLibrary.PrintString` (`KismetStringLibrary.Concat_StrStr` "State: " (`|GetEnumeratorNameAsString` (`self.AiState`)) " \nTask: " (`KismetSystemLibrary.GetDisplayName` (`self.CurrentTask`)) " \nTaskFinderIndex: " (`KismetStringLibrary.Conv_IntToString` (`self.TaskFinderIndex`))) true true (struct :`G` 0.66 :`B` 1.0 :`A` 1.0) DeltaSeconds))

(fn `GetNearestWall`
  (set `self.CurrentTask` (`.ReturnValue` (`GameplayStatics.FindNearestActor` (`self.K2_GetActorLocation`) (`self.PotentialTasks`))))
  (`self.SetWorking`)
  (`KismetSystemLibrary.PrintString` "Hello"))

(fn `UserConstructionScript`
  (`parent.UserConstructionScript`))

(fn `WorkAssigned`
  (params (Tasks :type "Array of Actor Object Reference"))
  (set `self.PotentialTasks` Tasks)
  (`self.GetNearestWall`))