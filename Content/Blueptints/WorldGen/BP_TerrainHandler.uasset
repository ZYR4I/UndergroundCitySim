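; BP_TerrainHandler edits wall tiles in the world grid, lowering them to destroy them or toggling their color.
; Both functions use a wall's index to address its instance in the grid's GroundMeshes.
; DestroyWall sinks the instance to a fixed height and teleports the wall actor there at unit scale, always returning false.
; SetWallColor switches a per-instance custom data value on or off, printing the result.
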(fn `DestroyWall`
  (params (WallRef :type "/Game/Blueptints/WorldGen/BP_EnhancedWallCollision Object Reference"))
  (returns (ReturnValue :type Boolean))
  (bind _index (`MyWallCollision.Index` WallRef))
  (bind _groundmeshes (`MyTerrainGen.groundMeshes` (`self.GridRef`)))
  (bind _outinstancetransform (`InstancedStaticMeshComponent.GetInstanceTransform` _groundmeshes _index true))
  (bind _returnvalue (`KismetMathLibrary.MakeTransform` (`KismetMathLibrary.MakeVector` (.x (.location _outinstancetransform)) (.y (.location _outinstancetransform)) -400.0) (.rotation _outinstancetransform) (.scale _outinstancetransform)))
  (bind _returnvalue_2 (`InstancedStaticMeshComponent.UpdateInstanceTransform` _groundmeshes _index _returnvalue true true true))
  (if _returnvalue_2
    (`self.K2_SetActorTransform` WallRef (`KismetMathLibrary.MakeTransform` (.location _returnvalue) (.rotation _returnvalue)) false true))
  (return false))

(fn `SetWallColor`
  (params (InstanceIndex :type "/Game/Blueptints/WorldGen/BP_EnhancedWallCollision Object Reference") (`On?` :type Boolean))
  (`/Engine/EditorBlueprintResources/StandardMacros.IsValid` InstanceIndex
    (:`Is Valid`
      (bind _gridref (`self.GridRef`)
        (:`then`
          (bind _returnvalue (`InstancedStaticMeshComponent.SetCustomDataValue` (`MyTerrainGen.groundMeshes` _gridref) (`MyWallCollision.Index` InstanceIndex) 1 (`KismetMathLibrary.SelectFloat` 1.0 0.0 `On?`) true))
          (`KismetSystemLibrary.PrintString` (`KismetStringLibrary.Conv_BoolToString` _returnvalue))
          (return))
        (:`else`)))
    (:`Is Not Valid`
      (`KismetSystemLibrary.PrintString` "NotValid"))))

(fn `UserConstructionScript`)