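; Player controller that routes Enhanced Input to the player character for movement, camera rotation, zoom and clicking.
; On BeginPlay it adds the input mapping context, caches the BP_PlayerCharacter, then shows the cursor in Game and UI mode locked to the viewport.
; Each input action forwards straight to the matching function on the cached character, which holds the actual gameplay logic.
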(event `self.ReceiveBeginPlay`
  (`EnhancedInputSubsystemInterface.AddMappingContext` (subsystem `EnhancedInputLocalPlayerSubsystem`) "/Game/Iputs/IMC_MappingContext.IMC_MappingContext" 0 (struct))
  (bind _asbp_player_character (cast `/Game/Blueptints/Player/BP_PlayerCharacter` (`GameplayStatics.GetPlayerCharacter` 0)))
  (set `self.PlayerRef` _asbp_player_character)
  (set `self.bShowMouseCursor` true)
  (`WidgetBlueprintLibrary.SetInputMode_GameAndUIEx` self null "LockAlways" false))

(event `EnhancedInput|/Game/Iputs/Actions/IA_Move`
  (params (ActionValue :type "Vector2D Structure") (ElapsedSeconds :type "Float (double-precision)") (TriggeredSeconds :type "Float (double-precision)") (InputAction :type "InputAction Object Reference" :default "/Game/Iputs/Actions/IA_Move.IA_Move"))
  (:`Triggered`
    (`/Game/Blueptints/Player/BP_PlayerCharacter.Move` (`self.PlayerRef`) ActionValue_X ActionValue_Y)))

(event `EnhancedInput|/Game/Iputs/Actions/IA_RotateCamera`
  (params (ActionValue :type "Float (double-precision)") (ElapsedSeconds :type "Float (double-precision)") (TriggeredSeconds :type "Float (double-precision)") (InputAction :type "InputAction Object Reference" :default "/Game/Iputs/Actions/IA_RotateCamera.IA_RotateCamera"))
  (:`Triggered`
    (`/Game/Blueptints/Player/BP_PlayerCharacter.RotateCamera` (`self.PlayerRef`) ActionValue)))

(event `EnhancedInput|/Game/Iputs/Actions/IA_Zoom`
  (params (ActionValue :type "Float (double-precision)") (ElapsedSeconds :type "Float (double-precision)") (TriggeredSeconds :type "Float (double-precision)") (InputAction :type "InputAction Object Reference" :default "/Game/Iputs/Actions/IA_Zoom.IA_Zoom"))
  (:`Triggered`
    (`/Game/Blueptints/Player/BP_PlayerCharacter.ZoomCamera` (`self.PlayerRef`) ActionValue)))

(event `EnhancedInput|/Game/Iputs/Actions/IA_Click`
  (params (ActionValue :type Boolean) (ElapsedSeconds :type "Float (double-precision)") (TriggeredSeconds :type "Float (double-precision)") (InputAction :type "InputAction Object Reference" :default "/Game/Iputs/Actions/IA_Click.IA_Click"))
  (:`Triggered`
    (`/Game/Blueptints/Player/BP_PlayerCharacter.Click` (`self.PlayerRef`))))

(fn `UserConstructionScript`)